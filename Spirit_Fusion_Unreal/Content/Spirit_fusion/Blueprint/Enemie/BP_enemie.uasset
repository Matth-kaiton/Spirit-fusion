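; BP_enemie is an enemy actor with health, a floating health bar and an explosive death.
; BeginPlay caches the Health_bar widget from the HealBar component.
; Tick sets the bar's fill from the health ratio and rotates it to face the player camera.
; AnyDamage subtracts health and, when it runs out, triggers death, which spawns an enlarged explosion emitter at the mesh and destroys the actor.
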(event Custom|death
  (Effects|SpawnEmitteratLocation "/Game/StarterContent/Particles/P_Explosion.P_Explosion" (Transformation|GetWorldLocation (Variables|Character|GetMesh)) "0, 0, 0" "3.000000,3.000000,3.000000")
  (Actor|DestroyActor))

(event Game|Damage|EventAnyDamage
  (params (Damage :type Float%20%28single-precision%29) (DamageType :type Damage%20Type%20Object%20Reference) (InstigatedBy :type Controller%20Object%20Reference) (DamageCauser :type Actor%20Object%20Reference))
  (if (> (Variables|Health|GetHealth) 0.0)
    (bind _output_get (Variables|Health|SetHealth (- (Variables|Health|GetHealth) Damage)))
    (if (<= _output_get 0.0)
      (CallFunction|Death))))

(event EventBeginPlay
  (bind _ashealth_bar (Utilities|Casting|CastToHealth_bar (UserInterface|GetUserWidgetObject (Variables|HealtBar|Getheal_bar))))
  (Variables|healtBar|SetAs%20Health%20Bar _ashealth_bar))

(event EventTick
  (params (DeltaSeconds :type Float%20%28single-precision%29))
  (bind _heal_bar (Variables|HealtBar|Getheal_bar))
  (Progress|SetPercent (Variables|/Game/Spirit_fusion/Blueprint/Health_bar.Health_bar_C|GetProgressBar_0 (Variables|healtBar|GetAs%20Health%20Bar)) (/ (Variables|Health|GetHealth) (Variables|Health|GetmaxHealth)))
  (Transformation|SetWorldRotation _heal_bar (Math|Rotator|FindLookatRotation (Transformation|GetWorldLocation _heal_bar) (Transformation|GetWorldLocation (Variables|/Script/Engine.PlayerCameraManager|GetTransformComponent (Game|GetPlayerCameraManager 0)))) false false))

(fn ConstructionScript)