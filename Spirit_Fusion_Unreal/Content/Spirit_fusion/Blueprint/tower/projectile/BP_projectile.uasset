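; Tower projectile that homes in on a target and damages BP_enemie actors it hits.
; On BeginPlay with a valid Target, it aims velocity and rotation at it, sets the movement component's homing target and self-destructs after a timed delay.
; Box overlap casts the sweep's hit actor to BP_enemie, then spawns an explosion, calls DestroyActor and applies fixed damage afterward.
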(event OnComponentBeginOverlap(Box)
  (params (OverlappedComponent :type Primitive%20Component%20Object%20Reference) (OtherActor :type Actor%20Object%20Reference) (OtherComp :type Primitive%20Component%20Object%20Reference) (OtherBodyIndex :type Integer) (bFromSweep :type Boolean) (SweepResult :type Hit%20Result%20Structure%20%28by%20ref%29))
  (bind _hitactor (Collision|BreakHitResult SweepResult))
  (bind _asbp_enemie (Utilities|Casting|CastToBP_enemie _hitactor))
  (if (== _asbp_enemie _hitactor)
    (Effects|SpawnEmitteratLocation "/Game/StarterContent/Particles/P_Explosion.P_Explosion" (Transformation|GetActorLocation _hitactor) "0, 0, 0" "5.000000,5.000000,5.000000")
    (Actor|DestroyActor)
    (Actor|GetActorOfClass "/Game/Spirit_fusion/Blueprint/Enemie/BP_enemie.BP_enemie_C")
    (Game|Damage|ApplyDamage _hitactor 35.0 0 0)))

(event Custom|Aim%20at%20target
  (bind _output_get (Variables|/Script/Engine.MovementComponent|SetVelocity (Variables|Default|Getmovement) (Math|Vector|GetUnitDirection(Vector) (Transformation|GetActorLocation) (Transformation|GetActorLocation (Variables|Default|Gettarget)))))
  (Transformation|SetActorRotation (Math|Conversions|RotationFromXVector _output_get)))

(event EventBeginPlay
  (Variables|Default|Gettarget
    (:then
      (CallFunction|AimatTarget)
      (Variables|/Script/Engine.ProjectileMovementComponent|SetHomingTargetComponent (Variables|Default|Getmovement) (Variables|/Script/Engine.Actor|GetRootComponent (Variables|Default|Gettarget)))
      (Utilities|FlowControl|Delay 1e+01)
      (Actor|DestroyActor))
    (:else)))

(fn ConstructionScript)