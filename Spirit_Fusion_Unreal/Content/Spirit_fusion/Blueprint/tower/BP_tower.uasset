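; Tower actor that attacks BP_enemie actors that overlap it, one target at a time.
; An overlap counter lets an arriving actor become the target only when no others are counted.
; Hitter then subtracts fixed health on a recursive delay loop, destroying the enemy at zero.
; Any end overlap flags out of range, halting the loop; DealDammage and the construction script are empty.
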(event Custom|Hitter
  (if (not (Variables|Default|GetNot_In_Range))
    (bind _asbp_enemie (Utilities|Casting|CastToBP_enemie (Variables|Default|Getenemie)))
    (if (> (Variables|/Game/Spirit_fusion/Blueprint/Enemie/BP_enemie.BP_enemie_C|Gethealth_enemie _asbp_enemie) 0.0)
      (Variables|/Game/Spirit_fusion/Blueprint/Enemie/BP_enemie.BP_enemie_C|Sethealth_enemie _asbp_enemie (- (Variables|/Game/Spirit_fusion/Blueprint/Enemie/BP_enemie.BP_enemie_C|Gethealth_enemie _asbp_enemie) 5e+01))
      (if (> (Variables|/Game/Spirit_fusion/Blueprint/Enemie/BP_enemie.BP_enemie_C|Gethealth_enemie _asbp_enemie) 0.0)
        (Utilities|FlowControl|Delay 0.5)
        (CallFunction|Hitter)
        (else
          (Actor|DestroyActor _asbp_enemie)
          (Variables|Default|Setenemi_count (- (Variables|Default|Getenemi_count) 1))))
      (else
        (Actor|DestroyActor _asbp_enemie)))))

(event Collision|EventActorEndOverlap
  (params (OtherActor :type Actor%20Object%20Reference))
  (Variables|Default|SetNot_In_Range true)
  (Variables|Default|Setenemi_count (- (Variables|Default|Getenemi_count) 1)))

(event Collision|EventActorBeginOverlap
  (params (OtherActor :type Actor%20Object%20Reference))
  (bind _output_get (Variables|Default|Setenemi_count (+ (Variables|Default|Getenemi_count) 1)))
  (if (<= _output_get 1)
    (Variables|Default|Setenemie OtherActor)
    (Variables|Default|SetNot_In_Range false)
    (CallFunction|Hitter)))

(fn ConstructionScript)

(fn DealDammage
  (params (Ennemyhit :type Actor%20Object%20Reference)))